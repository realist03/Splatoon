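; Player pawn that paints hit masks with the mouse in a Splatoon-style setup, showing the cursor at start.
; While the left mouse button is held, Tick runs a complex Visibility trace under the cursor.
; When the hit actor is a BP_HitMask, the pawn passes it the hit location and calls HitTestMask on it.
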(event EventBeginPlay
  (Variables|/Script/Engine.PlayerController|SetbShowMouseCursor (Game|GetPlayerController 0) true)
  (bind _outactors (Actor|GetAllActorsOfClass "BP_HitMask_Pawn_C"))
  (Variables|BP_HitMask_Pawn_C|SetBP_HitMask_Pawn (Utilities|Array|Get(acopy) _outactors) 0))

(event EventTick
  (params (DeltaSeconds :type Float%20%28single-precision%29))
  (if (Variables|Default|GetPressed)
    (bind _hitactor (CallFunction|LineTraceUnderCursor))
    (bind _asbp_hit_mask (Utilities|Casting|CastToBP_HitMask _hitactor))
    (Variables|/Game/Splatoon/BP_HitMask.BP_HitMask_C|SetHitPoint _asbp_hit_mask (Variables|Default|GetHitPoint))
    (Default|HitTestMask _asbp_hit_mask)))

(event Input|MouseEvents|LeftMouseButton
  (params (Key :type Key%20Structure))
  (:Pressed
    (Variables|Default|SetPressed true))
  (:Released
    (Variables|Default|SetPressed false)))

(fn ConstructionScript)

(fn LineTraceUnderCursor
  (bind _returnvalue (Game|GetPlayerController 0))
  (bind (_hitresult _returnvalue_2) (Game|Player|GetHitResultUnderCursorbyChannel _returnvalue "TraceTypeQuery1" true))
  (bind (_bblockinghit _binitialoverlap _time _distance _location _impactpoint _normal _impactnormal _physmat _hitactor) (Collision|BreakHitResult _hitresult))
  (if _returnvalue_2
    (Variables|Default|SetHitPoint _location)
    (bind _output_get (Variables|Default|SetHitActor _hitactor)))
  (return _output_get))