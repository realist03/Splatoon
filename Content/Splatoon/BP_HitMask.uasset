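; Splatoon-style hit mask actor that records a hit point on its mesh into the RT_HitMask render target, cleared on BeginPlay.
; HitTestMask briefly swaps the mesh to an unwrap material for a scene capture of only this actor, then switches it to M_HitMask.
; It then passes HitPoint to a dynamic instance of M_Damage_Inst and draws that into RT_HitMask, printing the point for debug.
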(event Custom|HitTestMask
  (bind _hitpoint (Variables|Default|GetHitPoint))
  (Rendering|Material|SetMaterial (Variables|Debug|GetStaticMeshComponent) 0 "/Game/Splatoon/M_RT_UnWrap_Mat_Inst.M_RT_UnWrap_Mat_Inst")
  (Rendering|SceneCapture|CaptureScene (Variables|Default|GetSceneCaptureComponent2D) :!class /Script/Engine.SceneCaptureComponent2D)
  (Rendering|Material|SetMaterial (Variables|Debug|GetStaticMeshComponent) 0 "/Game/Splatoon/M_HitMask.M_HitMask")
  (Development|PrintString (Utilities|String|ToString(Vector) _hitpoint))
  (Rendering|Material|SetVectorParameterValue (Variables|Default|GetHitMask) "P" (Math|Conversions|ToLinearColor(Vector) _hitpoint) :!class /Script/Engine.MaterialInstanceDynamic)
  (Rendering|DrawMaterialtoRenderTarget "/Game/Splatoon/RT_HitMask.RT_HitMask" (Variables|Default|GetHitMask)))

(event EventBeginPlay
  (bind _returnvalue (Rendering|Material|CreateDynamicMaterialInstance "/Game/Splatoon/M_Damage_Inst.M_Damage_Inst" "None" :!class /Script/Engine.KismetMaterialLibrary))
  (Variables|Default|SetHitMask _returnvalue)
  (Variables|/Script/Engine.SceneCaptureComponent|SetShowOnlyActors (Variables|Default|GetSceneCaptureComponent2D) (Utilities|Array|MakeArray self))
  (Rendering|ClearRenderTarget2D "/Game/Splatoon/RT_HitMask.RT_HitMask"))

(event Collision|EventActorBeginOverlap
  (params (OtherActor :type Actor%20Object%20Reference)))

(event EventTick
  (params (DeltaSeconds :type Float%20%28single-precision%29)))

(fn ConstructionScript)